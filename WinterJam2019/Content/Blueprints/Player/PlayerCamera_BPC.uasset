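; Player camera component that drives field of view through stackable, keyed multipliers.
; It caches the starting FOV on BeginPlay, then every tick multiplies it by all values in the FOVMultiplierQueue map and applies the result.
; UpdateFOVQueue writes a multiplier under its key, while LerpFOVQueue blends from 1.0 toward the given multiplier by Alpha before writing it, allowing effects to fade.
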(event EventBeginPlay
  (Variables|Default|SetCached%20Field%20Of%20View (Variables|Default|GetFieldOfView)))

(event EventTick
  (params (DeltaSeconds :type Float%20%28single-precision%29))
  (CallFunction|UpdateFieldOfView))

(fn UpdateFieldOfView
  (bind _fov_multiplier_queue (Variables|Default|GetFOV%20Multiplier%20Queue))
  (LocalVariables|SetAccumulated%20Field%20Of%20View (Variables|Default|GetCached%20Field%20Of%20View))
  (bind _keys (Utilities|Map|Keys _fov_multiplier_queue))
  (for _array_element _keys
    (if (.ReturnValue (Utilities|Map|Find _fov_multiplier_queue _array_element))
      (|SetBy-RefVar (LocalVariables|GetAccumulated%20Field%20Of%20View) (* (LocalVariables|GetAccumulated%20Field%20Of%20View) (.Value (Utilities|Map|Find _fov_multiplier_queue _array_element))))))
  (Camera|SetFieldOfView (LocalVariables|GetAccumulated%20Field%20Of%20View)))

(fn UpdateFOVQueue
  (params (Key :type F%20Camera%20FOV%20Queue%20Element%20Structure))
  (Utilities|Map|Add (Variables|Default|GetFOV%20Multiplier%20Queue) (.key Key) (.fovmultiplier Key))
  (return (.key Key)))

(fn LerpFOVQueue
  (params (Key :type F%20Camera%20FOV%20Queue%20Element%20Structure) (Alpha :type Float%20%28single-precision%29))
  (bind _returnvalue (Math|Float|Lerp 1.0 (.fovmultiplier Key) Alpha))
  (bind _out_key (CallFunction|UpdateFOVQueue (Utilities|Struct|MakeFCameraFOVQueueElement (.key Key) _returnvalue)))
  (return _out_key _returnvalue))