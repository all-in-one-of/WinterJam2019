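; Attribute_BPC is a player component that holds a single numeric attribute bounded between zero and a maximum.
; SetValue clamps the new value, fires a full or empty event at either bound, then always fires a set event.
; AddValue applies non-zero deltas through SetValue and then fires an added event.
; IsEmpty and IsFull report whether the value sits at either bound, and Tick is unused.
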(event EventTick
  (params (DeltaSeconds :type Float%20%28single-precision%29)))

(fn SetValue
  (params (New%20Value :type Float%20%28single-precision%29))
  (Utilities|FlowControl|Sequence
    (:then_0
      ;[1 0.9412 0] Clamp
      (Variables|Attribute|SetValue (Math|Float|Clamp(Float) New%20Value 0.0 (Variables|Attribute|GetMax%20Value))))
    (:then_1
      (if (>= (Variables|Attribute|GetValue) (Variables|Attribute|GetMax%20Value))
        (Default|CallOnValueFull)
        (elif (<= (Variables|Attribute|GetValue) 0.0)
          (Default|CallOnValueEmpty))))
    (:then_2
      (Default|CallOnValueSet))))

(fn AddValue
  (params (Delta :type Float%20%28single-precision%29))
  (if (!= Delta 0.0)
    (Utilities|FlowControl|Sequence
      (:then_0
        (Attribute|SetValue (+ (Variables|Attribute|GetValue) Delta)))
      (:then_1
        (Default|CallOnValueAdded)))))

(fn IsEmpty
  (return (<= (Variables|Attribute|GetValue) 0.0)))

(fn IsFull
  (return (>= (Variables|Attribute|GetValue) (Variables|Attribute|GetMax%20Value))))