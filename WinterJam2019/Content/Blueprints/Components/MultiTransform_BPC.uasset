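; Scene component that layers several transform offsets on top of its starting relative transform, letting multiple sources drive one relative transform.
; It caches the relative transform on BeginPlay, then every Tick folds the Transforms array onto it and sets the result.
; Locations are summed, rotations combined and scales multiplied separately, rather than composed as full transforms.
; Callers register an offset with AddTransform, which returns its index, and change it through SetTransformByIndex.
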(event EventBeginPlay
  (Variables|MultiTransform|SetCached%20Relative%20Transform (Transformation|GetRelativeTransform)))

(event EventTick
  (params (DeltaSeconds :type Float%20%28single-precision%29))
  (MultiTransform|UpdateRelativeTransform))

(fn UpdateRelativeTransform
  (LocalVariables|SetAccumulated%20Transform (Variables|MultiTransform|GetCached%20Relative%20Transform))
  (for _array_element (Variables|MultiTransform|GetTransforms)
    (LocalVariables|SetAccumulated%20Transform (Math|Transform|MakeTransform (+ (.location (LocalVariables|GetAccumulated%20Transform)) (.location _array_element)) (Math|Rotator|CombineRotators (.rotation (LocalVariables|GetAccumulated%20Transform)) (.rotation _array_element)) (* (.scale _array_element) (.scale (LocalVariables|GetAccumulated%20Transform))))))
  (Transformation|SetRelativeTransform (LocalVariables|GetAccumulated%20Transform) false false))

(fn AddTransform
  (params (Transform :type Transform))
  (bind _transforms (Variables|MultiTransform|GetTransforms))
  (bind _returnvalue (Utilities|Array|Add _transforms Transform))
  (return (Utilities|Array|Get(acopy) _transforms _returnvalue) _returnvalue))

(fn SetTransformbyIndex
  (params (Index :type Integer) (Transform :type Transform))
  (Utilities|Array|SetArrayElem (Variables|MultiTransform|GetTransforms) Index Transform))