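; Scene component that blends its relative transform from the one cached at BeginPlay toward a target.
; SetTargetLocation, SetTargetRotation and SetTargetScale each store target, settings and alpha, then apply a lerp from the cached value.
; Per-axis settings choose Ignore, Replace or Additive, with Additive summing location, combining rotators and multiplying scale.
; Lerping always from the cached transform makes alpha an absolute blend rather than an accumulating step.
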(event EventBeginPlay
  (Variables|Default|SetCached%20Relative%20Transform (Transformation|GetRelativeTransform)))

(fn GetSingleVectorSettings
  (params (Selection :type ETransformToTargetMode%20Enum :default "NewEnumerator0") (Cached :type Float%20%28single-precision%29) (Target :type Float%20%28single-precision%29) (Add%20or%20Multiply :type Boolean))
  (switch Utilities|FlowControl|Switch|SwitchonETransformToTargetMode Selection
    (:NewEnumerator0
      (return Cached))
    (:NewEnumerator1
      (return Target))
    (:NewEnumerator2
      (return (Math|Float|SelectFloat (* Cached Target) (+ Cached Target) Add%20or%20Multiply)))))

(fn GetRotationSettings
  (bind _cached_relative_transform (Variables|Default|GetCached%20Relative%20Transform))
  (bind _target (Variables|Default|GetTarget))
  (bind _settings (Variables|Default|GetSettings))
  (bind _returnvalue (Math|Rotator|CombineRotators (.rotation _cached_relative_transform) (.rotation _target)))
  (bind (_roll _pitch _yaw) (Math|Rotator|BreakRotator (.rotation _target)))
  (bind (_roll_2 _pitch_2 _yaw_2) (Math|Rotator|BreakRotator (.rotation _cached_relative_transform)))
  (Utilities|FlowControl|Sequence
    (:then_0
      (switch Utilities|FlowControl|Switch|SwitchonETransformToTargetMode (.x (.rotation _settings))
        (:NewEnumerator0
          (LocalVariables|SetX _roll_2))
        (:NewEnumerator1
          (LocalVariables|SetX _roll))
        (:NewEnumerator2
          (LocalVariables|SetX (.roll _returnvalue)))))
    (:then_1
      (switch Utilities|FlowControl|Switch|SwitchonETransformToTargetMode (.y (.rotation _settings))
        (:NewEnumerator0
          (LocalVariables|SetY _pitch_2))
        (:NewEnumerator1
          (LocalVariables|SetY _pitch))
        (:NewEnumerator2
          (LocalVariables|SetY (.pitch _returnvalue)))))
    (:then_2
      (switch Utilities|FlowControl|Switch|SwitchonETransformToTargetMode (.z (.rotation _settings))
        (:NewEnumerator0
          (LocalVariables|SetZ _yaw_2))
        (:NewEnumerator1
          (LocalVariables|SetZ _yaw))
        (:NewEnumerator2
          (LocalVariables|SetZ (.yaw _returnvalue)))))
    (:then_3
      (return (Math|Rotator|MakeRotator (LocalVariables|GetX) (LocalVariables|GetY) (LocalVariables|GetZ))))))

(fn GetLocationSettings
  (bind _cached_relative_transform (Variables|Default|GetCached%20Relative%20Transform))
  (bind _target (Variables|Default|GetTarget))
  (bind _settings (Variables|Default|GetSettings))
  (return (Math|Vector|MakeVector (Calculation|GetSingleVectorSettings (.x (.location _settings)) (.x (.location _cached_relative_transform)) (.x (.location _target)) false) (Calculation|GetSingleVectorSettings (.y (.location _settings)) (.y (.location _cached_relative_transform)) (.y (.location _target)) false) (Calculation|GetSingleVectorSettings (.z (.location _settings)) (.z (.location _cached_relative_transform)) (.z (.location _target)) false))))

(fn GetScaleSettings
  (bind _returnvalue (Class|KismetSystemLibrary|MakeLiteralBool true))
  (bind _cached_relative_transform (Variables|Default|GetCached%20Relative%20Transform))
  (bind _target (Variables|Default|GetTarget))
  (bind _settings (Variables|Default|GetSettings))
  (return (Math|Vector|MakeVector (Calculation|GetSingleVectorSettings (.x (.scale _settings)) (.x (.scale _cached_relative_transform)) (.x (.scale _target)) _returnvalue) (Calculation|GetSingleVectorSettings (.y (.scale _settings)) (.y (.scale _cached_relative_transform)) (.y (.scale _target)) _returnvalue) (Calculation|GetSingleVectorSettings (.z (.scale _settings)) (.z (.scale _cached_relative_transform)) (.z (.scale _target)) _returnvalue))))

(fn SetTargetLocation
  (params (Target%20Location :type Vector) (Settings :type F%20Transform%20to%20Target%20Row%20Settings%20Structure) (Alpha :type Float%20%28single-precision%29))
  (Variables|Default|SetTarget (Math|Transform|MakeTransform Target%20Location (.rotation (Variables|Default|GetTarget)) (.scale (Variables|Default|GetTarget))))
  (bind _output_get (Variables|Interpolation|SetLocation%20Alpha Alpha))
  (Utilities|Struct|SetmembersinFTransformToTargetSettings (Variables|Default|GetSettings) Settings)
  (Transformation|SetRelativeLocation (Math|Vector|Lerp(Vector) (.location (Variables|Default|GetCached%20Relative%20Transform)) (Calculation|GetLocationSettings) _output_get) (Variables|Interpolation|GetSweep) (Variables|Interpolation|GetTeleport)))

(fn SetTargetScale
  (params (Target%20Scale :type Vector) (Settings :type F%20Transform%20to%20Target%20Row%20Settings%20Structure) (Alpha :type Float%20%28single-precision%29))
  (Variables|Default|SetTarget (Math|Transform|MakeTransform (.location (Variables|Default|GetTarget)) (.rotation (Variables|Default|GetTarget)) Target%20Scale))
  (bind _output_get (Variables|Interpolation|SetScale%20Alpha Alpha))
  (Utilities|Struct|SetmembersinFTransformToTargetSettings (Variables|Default|GetSettings) Settings)
  (Transformation|SetRelativeScale3D (Math|Vector|Lerp(Vector) (.scale (Variables|Default|GetCached%20Relative%20Transform)) (Calculation|GetScaleSettings) _output_get)))

(fn SetTargetRotation
  (params (Target%20Rotation :type Rotator) (Settings :type F%20Transform%20to%20Target%20Row%20Settings%20Structure) (Alpha :type Float%20%28single-precision%29))
  (Variables|Default|SetTarget (Math|Transform|MakeTransform (.location (Variables|Default|GetTarget)) Target%20Rotation (.scale (Variables|Default|GetTarget))))
  (bind _output_get (Variables|Interpolation|SetRotation%20Alpha Alpha))
  (Utilities|Struct|SetmembersinFTransformToTargetSettings (Variables|Default|GetSettings) Settings)
  (Transformation|SetRelativeRotation (Math|Rotator|Lerp(Rotator) (.rotation (Variables|Default|GetCached%20Relative%20Transform)) (Calculation|GetRotationSettings) _output_get (Variables|Interpolation|GetShortest%20Path)) false false))