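; Scene component that animates its relative transform over time, offsetting it from the BeginPlay transform toward TransformDelta using curves.
; Tick advances separate per-axis timers for location, rotation and scale, each at its own speed.
; SampleCurve works on fractional time for looping, and its per-axis alphas drive three-way lerps into SetRelativeTransform.
; As wired, rotation samples ScaleCurve and scale samples RotationCurve.
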(event EventBeginPlay
  ;[1 1 1] Init
  (Variables|Default|SetCached%20Relative%20Transform (Transformation|GetRelativeTransform))
  (Variables|Default|SetAccumulated%20Location%20Time (Math|Vector|MakeVector 0.0 0.0 0.0)))

(event EventTick
  (params (DeltaSeconds :type Float%20%28single-precision%29))
  (bind _transform_delta (Variables|Transform|GetTransform%20Delta))
  (bind _accumulated_scale_time (Variables|Default|GetAccumulated%20Scale%20Time))
  (bind _accumulated_rotation_time (Variables|Default|GetAccumulated%20Rotation%20Time))
  (bind _accumulated_location_time (Variables|Default|GetAccumulated%20Location%20Time))
  (bind _cached_relative_transform (Variables|Default|GetCached%20Relative%20Transform))
  (Utilities|FlowControl|Sequence
    (:then_0
      (Utilities|FlowControl|Sequence
        (:then_0
          (|SetBy-RefVar _accumulated_location_time (+ _accumulated_location_time (* (Variables|Transform|GetLocation%20Speed) (Utilities|Time|GetWorldDeltaSeconds)))))
        (:then_1
          (|SetBy-RefVar _accumulated_rotation_time (+ _accumulated_rotation_time (* (Variables|Transform|GetRotation%20Speed) (Utilities|Time|GetWorldDeltaSeconds)))))
        (:then_2
          (|SetBy-RefVar _accumulated_scale_time (+ _accumulated_scale_time (* (Variables|Transform|GetScale%20Speed) (Utilities|Time|GetWorldDeltaSeconds)))))))
    (:then_1
      (Transformation|SetRelativeTransform (Math|Transform|MakeTransform (CallFunction|Lerp(vector3-way) (.location _cached_relative_transform) (+ (.location _cached_relative_transform) (.location _transform_delta)) (Utilities|SampleCurve (Variables|Transform|GetLocation%20Curve) (Variables|Default|GetAccumulated%20Location%20Time))) (CallFunction|Lerp(rotator3-way) (.rotation _cached_relative_transform) (Math|Rotator|CombineRotators (.rotation _cached_relative_transform) (.rotation _transform_delta)) (Utilities|SampleCurve (Variables|Transform|GetScale%20Curve) (Variables|Default|GetAccumulated%20Rotation%20Time))) (CallFunction|Lerp(vector3-way) (.scale _cached_relative_transform) (+ (.scale _cached_relative_transform) (- (.scale _transform_delta) 1.0)) (Utilities|SampleCurve (Variables|Transform|GetRotation%20Curve) (Variables|Default|GetAccumulated%20Scale%20Time)))) (Variables|Transform|GetSweep) (Variables|Transform|GetTeleport)))))