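; EnemyBase_BP is a base enemy character Blueprint with health, damage and ragdoll death.
; ApplyDamage subtracts the damage from a Health component.
; When Health signals it is empty, a DoOnce triggers Kill, which zeroes health, disables capsule collision and turns on mesh physics with query and physics collision.
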(event OnValueEmpty(Health)
  (Utilities|FlowControl|DoOnce false
    (:Completed
      (Attributes|Kill))))

(event EventBeginPlay)

(event Collision|EventActorBeginOverlap
  (params (OtherActor :type Actor%20Object%20Reference)))

(event EventTick
  (params (DeltaSeconds :type Float%20%28single-precision%29)))

(fn ConstructionScript)

(fn Kill
  (bind _mesh (Variables|Character|GetMesh))
  (Utilities|FlowControl|Sequence
    (:then_0
      (Default|SetValue (Variables|Default|GetHealth) 0.0))
    (:then_1
      (Collision|SetCollisionEnabled (Variables|Collision|GetCapsuleComponent) "NoCollision"))
    (:then_2
      (Physics|SetSimulatePhysics _mesh true)
      (Collision|SetCollisionEnabled _mesh "QueryAndPhysics"))))

(fn ApplyDamage
  (params (Damage :type Float%20%28single-precision%29))
  (Default|AddValue (Variables|Default|GetHealth) (* Damage -1.0)))