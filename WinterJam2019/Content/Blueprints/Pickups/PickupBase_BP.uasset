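; Base pickup actor that reacts when the player touches it, playing a sound and destroying itself.
; Trigger overlap filters for Player_BP, stores the sweep hit and player, then calls the OnPlayerEntereredProximity event.
; That event plays the configured Sound struct at the stored hit location, if its sound is valid, then destroys the actor.
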(event OnComponentBeginOverlap(Trigger)
  (params (OverlappedComponent :type Primitive%20Component%20Object%20Reference) (OtherActor :type Actor%20Object%20Reference) (OtherComp :type Primitive%20Component%20Object%20Reference) (OtherBodyIndex :type Integer) (bFromSweep :type Boolean) (SweepResult :type Hit%20Result%20Structure%20%28by%20ref%29))
  (bind _asplayer_bp (Utilities|Casting|CastToPlayer_BP OtherActor))
  (Variables|Default|SetHit SweepResult)
  (bind _output_get (Variables|Default|SetPlayer%20To%20Follow _asplayer_bp))
  (CallFunction|OnPlayerEntereredProximity _output_get))

(event Custom|OnPlayerEntereredProximity
  (params (Player :type Player%20BP%20Object%20Reference))
  (bind _sound (Variables|Default|GetSound))
  (Utilities|FlowControl|Sequence
    (:then_0
      (Utilities|IsValid (.sound _sound)
        (:Is%20Valid
          (Audio|PlaySoundatLocation (.sound _sound) (.location (Variables|Default|GetHit)) "0, 0, 0" (.volumemultiplier _sound) (.pitchmultiplier _sound) 0.0 (.attenuationsettings _sound) 0 Player))))
    (:then_1
      (Actor|DestroyActor))))

(event EventBeginPlay)

(event Collision|EventActorBeginOverlap
  (params (OtherActor :type Actor%20Object%20Reference)))

(event EventTick
  (params (DeltaSeconds :type Float%20%28single-precision%29)))

(fn ConstructionScript)