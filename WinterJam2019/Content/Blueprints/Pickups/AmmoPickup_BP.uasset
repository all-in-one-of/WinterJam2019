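; Ammo pickup Blueprint that refills a player's ammo pool when the player enters its proximity.
; It looks up the player's pool for its ammo type and adds its ammo amount only if that pool exists and is not full.
; The parent's proximity handler runs only after a successful refill, so players without a matching pool or with full ammo do not trigger it.
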(event EventBeginPlay
  (|CallParentFunction) ; This node is disabled and will not be called.\nDrag off pins to build functionality.
)

(event Collision|EventActorBeginOverlap
  (params (OtherActor :type Actor%20Object%20Reference))
  (|CallParentFunction OtherActor) ; This node is disabled and will not be called.\nDrag off pins to build functionality.
)

(event EventTick
  (params (DeltaSeconds :type Float%20%28single-precision%29))
  (|CallParentFunction DeltaSeconds) ; This node is disabled and will not be called.\nDrag off pins to build functionality.
)

(event EventOnPlayerEntereredProximity
  (params (Player :type Player%20BP%20Object%20Reference))
  (bind _ammo_type (Variables|Default|GetAmmo%20Type))
  (bind _ammo_pool (Default|GetAmmoPoolfromClass Player _ammo_type))
  (Utilities|IsValid _ammo_pool
    (:Is%20Valid
      (if (not (Default|IsAmmoFull _ammo_pool))
        (Default|AddtoCurrentAmmo _ammo_pool (Variables|Default|GetAmmo))
        (|CallParentFunction Player)))))

(fn ConstructionScript
  (|CallParentFunction))