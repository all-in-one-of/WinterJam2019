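; CollisionVolume_BP is a tool actor that provides a collision volume with a selectable pivot.
; Its construction script offsets the Collision component vertically by its bounds' Z extent, down for a Top pivot or up for a Bottom pivot.
; It then copies the actor's scale into the component's relative scale, after the offset has been computed.
; The event graph holds no active logic.
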(event EventBeginPlay)

(event Collision|EventActorBeginOverlap
  (params (OtherActor :type Actor%20Object%20Reference)))

(event EventTick
  (params (DeltaSeconds :type Float%20%28single-precision%29)))

(fn ConstructionScript
  (bind _collision (Variables|Default|GetCollision))
  (Utilities|FlowControl|Sequence
    (:then_0
      (switch Utilities|FlowControl|Switch|SwitchonEPivotMode (Variables|Default|GetPivot)
        (:NewEnumerator1
          (Transformation|SetRelativeLocation _collision (Math|Vector|MakeVector 0.0 0.0 (CallFunction|Invert (.z (.BoxExtent (Collision|GetComponentBounds _collision))))) false false))
        (:NewEnumerator2
          (Transformation|SetRelativeLocation _collision (Math|Vector|MakeVector 0.0 0.0 (.z (.BoxExtent (Collision|GetComponentBounds _collision)))) false false))))
    (:then_1
      (Transformation|SetRelativeScale3D (Variables|Default|GetCollision) (Transformation|GetActorScale3D)))))