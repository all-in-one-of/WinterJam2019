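; KitMesh_BP is a tool actor that displays one static mesh selected from grouped mesh lists by two indices.
; Its construction script clamps ListIndex and MeshIndex to valid ranges, then applies the GetStaticMesh result to the StaticMeshComponent.
; GetStaticMesh looks up the selected list's StaticMeshes entry, and the event graph holds only disabled stubs, so the Blueprint adds no runtime logic.
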(event EventBeginPlay
  (|CallParentFunction) ; This node is disabled and will not be called.\nDrag off pins to build functionality.
)

(event Collision|EventActorBeginOverlap
  (params (OtherActor :type Actor%20Object%20Reference))
  (|CallParentFunction OtherActor) ; This node is disabled and will not be called.\nDrag off pins to build functionality.
)

(event EventTick
  (params (DeltaSeconds :type Float%20%28single-precision%29))
  (|CallParentFunction DeltaSeconds) ; This node is disabled and will not be called.\nDrag off pins to build functionality.
)

(fn ConstructionScript
  (bind _mesh_list (Variables|StaticMesh|GetMesh%20List))
  (bind _mesh_index (Variables|StaticMesh|GetMesh%20Index))
  (bind _list_index (Variables|StaticMesh|GetList%20Index))
  (Utilities|FlowControl|Sequence
    (:then_0
      ;[0.1779 1 0.8802] Clamp indices
      (|SetBy-RefVar _list_index (Math|Integer|Clamp(Integer) _list_index 0 (Utilities|Array|LastIndex _mesh_list)))
      (|SetBy-RefVar _mesh_index (Math|Integer|Clamp(Integer) _mesh_index 0 (Utilities|Array|LastIndex (.staticmeshes (Utilities|Array|Get(acopy) _mesh_list _list_index))))))
    (:then_1
      (Components|StaticMesh|SetStaticMesh (Variables|Default|GetStaticMeshComponent) (StaticMesh|GetStaticMesh)))
    (:then_2
      (|CallParentFunction))))

(fn GetStaticMesh
  (return (Utilities|Array|Get(acopy) (.staticmeshes (Utilities|Array|Get(acopy) (Variables|StaticMesh|GetMesh%20List) (Variables|StaticMesh|GetList%20Index))) (Variables|StaticMesh|GetMesh%20Index))))