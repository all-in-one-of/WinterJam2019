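; Base spline tool actor whose construction script rebuilds its spline through a shared Construct step.
; Construct can snap points onto surfaces with downward line traces and debug arrows, then force a point type, optionally including endpoints.
; StealPoints, with undo support, clears the spline and refills it from another actor's first spline component.
; Helpers set all point types when forcing is off, or refresh and reconstruct the spline.
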(event EventBeginPlay
  (|CallParentFunction))

(fn ConstructionScript
  (|CallParentFunction)
  (Spline|Utility|Construct))

(fn StealPoints
  (bind _spline (Variables|Default|GetSpline))
  (bind _steal_points_from_actor (Variables|Spline|GetSteal%20Points%20From%20Actor))
  (bind _returnvalue (Actor|GetComponentsByClass _steal_points_from_actor "/Script/Engine.SplineComponent"))
  (bind _output (Utilities|Array|Get(acopy) _returnvalue))
  (bind _returnvalue_2 (Spline|GetNumberOfSplinePoints _output))
  (bind _returnvalue_3 (- _returnvalue_2 1))
  ;[1 1 1] If there is a spline to steal from
  (if (!= (Variables|Spline|GetSteal%20Points%20From%20Actor) 0)
    (if (!= _output 0)
      (Development|Editor|CreateCopyforUndoBuffer self)
      (Utilities|FlowControl|Sequence
        (:then_0
          (Spline|ClearSplinePoints (Variables|Default|GetSpline) true)
          (for _index (range (Class|KismetSystemLibrary|MakeLiteralInteger) _returnvalue_3)
            (Utilities|FlowControl|Sequence
              (:then_0
                (Spline|AddSplinePoint _spline (Spline|GetLocationatSplinePoint _output _returnvalue_3 "Local") "Local" false))
              (:then_1
                (Spline|SetSplinePointType _spline _returnvalue_3 (Class|SplineComponent|GetSplinePointType _output _returnvalue_3) false))
              (:then_2
                (Spline|SetTangentatSplinePoint _spline _returnvalue_3 (Spline|GetTangentatSplinePoint _output _returnvalue_3 "Local") "Local" false))
              (:then_3
                (Spline|SetTangentsatSplinePoint _spline _returnvalue_3 (Spline|GetArriveTangentatSplinePoint _output _returnvalue_3 "Local") (Spline|GetLeaveTangentatSplinePoint _output _returnvalue_3 "Local") "Local" false))
              (:then_4
                (Class|SplineComponent|SetUpVectoratSplinePoint _spline _returnvalue_3 (Class|SplineComponent|GetUpVectoratSplinePoint _output 0 "Local") "Local" false)))))
        (:then_1
          (Spline|Utility|RefreshSpline true))))))

(fn Construct
  (bind _force_end_point_types_ (Variables|Spline|PointType|GetForce%20End%20Point%20Types?))
  (Utilities|FlowControl|Sequence
    (:then_0
      (Spline|Utility|ConformtoSurface))
    (:then_1
      (if (Variables|Spline|PointType|GetForce%20Point%20Type?)
        (bind (_spline _index) (Utilities|ForEachSplinePoint (Math|Integer|SelectInt 0 1 _force_end_point_types_) (Math|Integer|SelectInt 1 2 _force_end_point_types_))
          (:LoopBody
            (Spline|SetSplinePointType _spline _index (Variables|Spline|PointType|GetPoint%20Type) false))
          (:Completed
            (Spline|UpdateSpline _spline)))))
    (:then_2
      (return true))))

(fn SetPointstoType
  (if (not (Variables|Spline|PointType|GetForce%20Point%20Type?))
    (bind (_spline _index) (Utilities|ForEachSplinePoint 0 1)
      (:LoopBody
        (Spline|SetSplinePointType _spline _index (Variables|Spline|PointType|GetPoint%20Type) false))
      (:Completed
        (Spline|Utility|RefreshSpline true)))))

(fn RefreshSpline
  (params (Construct :type Boolean))
  (Spline|UpdateSpline (Variables|Default|GetSpline))
  (if Construct
    (Spline|Utility|Construct))
  (return true))

(fn ReconstructSpline
  (Spline|Utility|RefreshSpline true))

(fn GetNearestPointatDistance
  (params (Distance :type Float%20%28single-precision%29))
  (for _index (range 0 (- (Spline|GetNumberOfSplinePoints (Variables|Default|GetSpline)) 2))
    (return _index) ; Return floored distance
  )
  (return (- (Spline|GetNumberOfSplinePoints (Variables|Default|GetSpline)) 1)) ; Else we are past the last point so return that
)

(fn ConformtoSurface
  (if (Variables|Spline|Conform|GetConform%20To%20Surface?)
    (for _index (range (Class|KismetSystemLibrary|MakeLiteralInteger) (- (Spline|GetNumberOfSplinePoints (Variables|Default|GetSpline)) 1))
      (bind (_outhit _returnvalue) (Collision|LineTraceForObjects (Math|Vector|MakeVector (.x (Spline|GetLocationatSplinePoint (Variables|Default|GetSpline) _index "World")) (.y (Spline|GetLocationatSplinePoint (Variables|Default|GetSpline) _index "World")) (+ (.z (Transformation|GetActorLocation)) (Variables|Spline|Conform|GetZ%20Offset))) (+ (Math|Vector|MakeVector (.x (Spline|GetLocationatSplinePoint (Variables|Default|GetSpline) _index "World")) (.y (Spline|GetLocationatSplinePoint (Variables|Default|GetSpline) _index "World")) (+ (.z (Transformation|GetActorLocation)) (Variables|Spline|Conform|GetZ%20Offset))) (Math|Vector|MakeVector 0.0 0.0 (CallFunction|Invert (Variables|Spline|Conform|GetTrace%20Distance)))) (Variables|Spline|Conform|GetTrace%20Types) (Variables|Spline|Conform|GetTrace%20Complex?) 0 "None" true "(R=1.000000,G=0.000000,B=0.000000,A=1.000000)" "(R=0.000000,G=1.000000,B=0.000000,A=1.000000)" 0.15))
      (if _returnvalue
        (Spline|SetLocationatSplinePoint (Variables|Default|GetSpline) _index (Math|Vector|MakeVector (.X (Math|Vector|BreakVector (Math|Vector|MakeVector (.x (Spline|GetLocationatSplinePoint (Variables|Default|GetSpline) _index "World")) (.y (Spline|GetLocationatSplinePoint (Variables|Default|GetSpline) _index "World")) (+ (.z (Transformation|GetActorLocation)) (Variables|Spline|Conform|GetZ%20Offset))))) (.Y (Math|Vector|BreakVector (Math|Vector|MakeVector (.x (Spline|GetLocationatSplinePoint (Variables|Default|GetSpline) _index "World")) (.y (Spline|GetLocationatSplinePoint (Variables|Default|GetSpline) _index "World")) (+ (.z (Transformation|GetActorLocation)) (Variables|Spline|Conform|GetZ%20Offset))))) (+ (+ (Variables|Spline|Conform|GetZ%20Offset) (.z (Spline|GetScaleatSplinePoint (Variables|Default|GetSpline) _index))) (.Z (Math|Vector|BreakVector (.location _outhit))))) "World" true)
        (Rendering|Debug|DrawDebugArrow (Math|Vector|MakeVector (.x (Spline|GetLocationatSplinePoint (Variables|Default|GetSpline) _index "World")) (.y (Spline|GetLocationatSplinePoint (Variables|Default|GetSpline) _index "World")) (+ (.z (Transformation|GetActorLocation)) (Variables|Spline|Conform|GetZ%20Offset))) (+ (Math|Vector|MakeVector (.x (Spline|GetLocationatSplinePoint (Variables|Default|GetSpline) _index "World")) (.y (Spline|GetLocationatSplinePoint (Variables|Default|GetSpline) _index "World")) (+ (.z (Transformation|GetActorLocation)) (Variables|Spline|Conform|GetZ%20Offset))) (Math|Vector|MakeVector 0.0 0.0 (CallFunction|Invert (Variables|Spline|Conform|GetTrace%20Distance)))) 5.0 "(R=0.484375,G=0.008726,B=0.000000,A=1.000000)" 0.5 2.5)))))