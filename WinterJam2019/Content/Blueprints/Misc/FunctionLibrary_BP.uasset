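; Blueprint function library of general-purpose math and utility helpers.
; Math helpers cover saturate, safe integer-to-float division, rotator clamping, per-axis vector and rotator lerps, and component-wise fraction and sine.
; By-ref operators add, subtract or flip a variable in place and return the result.
; Other helpers set a play rate from a desired duration and configure primitive collision in one call, applying a default response plus per-channel overrides.
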(fn VectorXY
  (params (Vector :type Vector) (Scale :type Float%20%28single-precision%29))
  (return (* (Math|Vector|Normalize (Math|Vector|MakeVector (.x Vector) (.y Vector) 0.0)) Scale)))

(fn OneMinus
  (params (in :type Float%20%28single-precision%29))
  (return (- 1.0 (Math|Saturate in (LocalVariables|Get__WorldContext)))))

(fn Saturate
  (params (In :type Float%20%28single-precision%29))
  (return (Math|Float|Clamp(Float) In)))

(fn Integer/Integer(Float)
  (params (A :type Integer) (B :type Integer))
  (if (== B 0)
    (return 0.0)
    (else
      (return (/ (Math|Conversions|ToFloat(Integer) A) (Math|Conversions|ToFloat(Integer) B))))))

(fn ClampRotator
  (params (In :type Rotator) (Min :type Rotator) (Max :type Rotator :default "360.000000,360.000000,360.000000"))
  (return (Math|Rotator|MakeRotator (Math|Float|Clamp(Float) (.roll In) (.roll Min) (.roll Max)) (Math|Float|Clamp(Float) (.pitch In) (.pitch Min) (.pitch Max)) (Math|Float|Clamp(Float) (.yaw In) (.yaw Min) (.yaw Max)))))

(fn +=
  (params (In :type Float%20%28single-precision%29%20%28by%20ref%29) (+ :type Float%20%28single-precision%29))
  (bind _returnvalue (+ In +))
  (|SetBy-RefVar In _returnvalue)
  (return _returnvalue))

(fn -=
  (params (In :type Float%20%28single-precision%29%20%28by%20ref%29) (- :type Float%20%28single-precision%29))
  (bind _returnvalue (- In -))
  (|SetBy-RefVar In _returnvalue)
  (return _returnvalue))

(fn Invert
  (params (In :type Float%20%28single-precision%29))
  (return (* In -1.0)))

(fn FlipBool
  (params (In :type Boolean%20%28by%20ref%29))
  (bind _returnvalue (not In))
  (|SetBy-RefVar In _returnvalue)
  (return _returnvalue))

(fn SetPlayDuration
  (params (Target :type Timeline%20Component%20Object%20Reference%20%28by%20ref%29) (New%20Duration :type Float%20%28single-precision%29))
  (Components|Timeline|SetPlayRate Target (/ 1.0 New%20Duration)))

(fn Lerp(vector3-way)
  (params (A :type Vector) (B :type Vector) (Alpha :type Vector))
  (return (Math|Vector|MakeVector (Math|Float|Lerp (.x A) (.x B) (.x Alpha)) (Math|Float|Lerp (.y A) (.y B) (.y Alpha)) (Math|Float|Lerp (.z A) (.z B) (.z Alpha)))))

(fn Lerp(rotator3-way)
  (params (A :type Rotator) (B :type Rotator) (Alpha :type Vector))
  (return (Math|Rotator|MakeRotator (Math|Float|Lerp (.roll A) (.roll B) (.x Alpha)) (Math|Float|Lerp (.pitch A) (.pitch B) (.y Alpha)) (Math|Float|Lerp (.yaw A) (.yaw B) (.z Alpha)))))

(fn Fraction(vector)
  (params (In :type Vector))
  (return (Math|Vector|MakeVector (Math|Float|Fraction (.x In)) (Math|Float|Fraction (.y In)) (Math|Float|Fraction (.z In)))))

(fn Sin(vector)
  (params (In :type Vector))
  (return (Math|Vector|MakeVector (Math|Trig|Sin(Radians) (.x In)) (Math|Trig|Sin(Radians) (.y In)) (Math|Trig|Sin(Radians) (.z In)))))

(fn SetPrimitiveCollision
  (params (Target :type Primitive%20Component%20Object%20Reference) (Collision%20Enabled :type ECollisionEnabled%20Enum :default "QueryAndPhysics") (Collision%20Channel :type ECollisionChannel%20Enum :default "ECC_WorldStatic") (Default%20Response :type ECollisionResponse%20Enum :default "ECR_Block") (Collision%20Responses :type Map%20of%20ECollisionChannel%20Enums%20to%20Bytes :default "ECC_WorldStatic") (CanCharacterStepUpOn :type ECanBeCharacterBase%20Enum :default "ECB_Yes"))
  (Utilities|FlowControl|Sequence
    (:then_0
      (Collision|SetCollisionEnabled Target Collision%20Enabled))
    (:then_1
      (Collision|SetCollisionObjectType Target Collision%20Channel))
    (:then_2
      (Collision|SetCollisionResponsetoAllChannels Target Default%20Response)
      (bind _enumvalue (|ForEachECollisionChannel)
        (:LoopBody
          (if (.ReturnValue (Utilities|Map|Find Collision%20Responses _enumvalue))
            (Collision|SetCollisionResponsetoChannel Target _enumvalue (.Value (Utilities|Map|Find Collision%20Responses _enumvalue)))))))
    (:then_3
      (Variables|/Script/Engine.PrimitiveComponent|SetCanCharacterStepUpOn Target CanCharacterStepUpOn))))