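; Static mesh Blueprint that applies per-instance material parameter overrides through dynamic material instances.
; The construction script calls InitializeDMI, which creates a dynamic instance for every material slot on the mesh.
; It then applies the scalar, vector and texture parameter arrays to all slots, looping over each dynamic material for textures.
; Vector values are converted from color to vector, and the event graph is unused.
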(event EventBeginPlay)

(event Collision|EventActorBeginOverlap
  (params (OtherActor :type Actor%20Object%20Reference)))

(event EventTick
  (params (DeltaSeconds :type Float%20%28single-precision%29)))

(fn ConstructionScript
  (CallFunction|InitializeDMI))

(fn InitializeDMI
  (bind _staticmeshcomponent (Variables|Debug|GetStaticMeshComponent))
  (for (_array_element _array_index) (Rendering|Material|GetMaterials (Variables|Debug|GetStaticMeshComponent))
    (Rendering|Material|CreateDynamicMaterialInstance (Variables|Debug|GetStaticMeshComponent) _array_index _array_element "None" :!class /Script/Engine.PrimitiveComponent))
  (Utilities|FlowControl|Sequence
    (:then_0
      (for _array_element_2 (Variables|Materials|GetScalar%20Parameters)
        (Rendering|Material|SetScalarParameterValueonMaterials _staticmeshcomponent (.name (.parameterinfo _array_element_2)) (.parametervalue _array_element_2))))
    (:then_1
      (for _array_element_3 (Variables|Materials|GetVector%20Parameters)
        (Rendering|Material|SetVectorParameterValueonMaterials _staticmeshcomponent (.name (.parameterinfo _array_element_3)) (Math|Conversions|ToVector(LinearColor) (.parametervalue _array_element_3)))))
    (:then_2
      (for _array_element_4 (Variables|Materials|GetTexture%20Parameters)
        (for _array_element_5 (Rendering|Material|GetMaterials _staticmeshcomponent)
          (bind _asmaterial_instance_dynamic (Utilities|Casting|CastToMaterialInstanceDynamic _array_element_5))
          (Rendering|Material|SetTextureParameterValue _asmaterial_instance_dynamic (.name (.parameterinfo _array_element_4)) (.parametervalue _array_element_4)))))))