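; Directional light component that publishes its lighting state to the Lighting_SPC parameter collection for materials to read.
; UpdateParameters writes the component's world forward vector as Light Direction and its colour times intensity as Light Colour, with that scaled colour's vector length packed into alpha.
; The event graph is empty, so the component does not call the update itself.
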(event EventBeginPlay)

(event EventTick
  (params (DeltaSeconds :type Float%20%28single-precision%29)))

(fn UpdateParameters
  (bind _returnvalue (Rendering|Components|Light|GetLightColor))
  (bind _intensity (Variables|Default|GetIntensity))
  (bind _returnvalue_2 (* _returnvalue _intensity))
  (bind (_r _g _b) (Math|Color|BreakColor _returnvalue_2))
  (Rendering|Material|SetVectorParameterValue "/Game/Art/Shaders/ParameterCollections/Lighting_SPC.Lighting_SPC" "Light Direction" (Math|Conversions|ToLinearColor(Vector) (Math|Rotator|GetRotationXVector (Transformation|GetWorldRotation))) :!class /Script/Engine.KismetMaterialLibrary)
  (Rendering|Material|SetVectorParameterValue "/Game/Art/Shaders/ParameterCollections/Lighting_SPC.Lighting_SPC" "Light Colour" (Utilities|Struct|MakeLinearColor _r _g _b (Math|Vector|VectorLength (Math|Conversions|ToVector(LinearColor) _returnvalue_2))) :!class /Script/Engine.KismetMaterialLibrary))