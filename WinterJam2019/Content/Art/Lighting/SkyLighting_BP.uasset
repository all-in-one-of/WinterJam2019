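; Sky lighting actor that keeps a directional light, sky light and skybox sphere in sync from one set of settings.
; Update runs on construction and BeginPlay, refreshing the directional light and matching the direction arrow's color to it.
; A dynamic skybox material takes the actor's yaw plus an offset, a tint, and the cubemap shared with the sky light.
; It also lifts a colour calibrator by its bounds and sets its world yaw.
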(event EventBeginPlay
  (CallFunction|Update))

(event Collision|EventActorBeginOverlap
  (params (OtherActor :type Actor%20Object%20Reference)))

(event EventTick
  (params (DeltaSeconds :type Float%20%28single-precision%29)))

(fn ConstructionScript
  (CallFunction|Update))

(fn Update
  (bind _skysphere (Variables|Default|GetSkySphere))
  (bind _colourcalibrator (Variables|Default|GetColourCalibrator))
  (bind _cubemap (Variables|Lighting|GetCubemap))
  (Utilities|FlowControl|Sequence
    (:then_0
      (Default|UpdateParameters (Variables|Default|GetDirectionalLight)))
    (:then_1
      (bind _returnvalue (Rendering|Material|CreateDynamicMaterialInstance _skysphere 0 (Rendering|Material|GetMaterial _skysphere 0) "None" :!class /Script/Engine.PrimitiveComponent))
      (bind _output_get (Variables|Lighting|SetSkybox%20DMI _returnvalue))
      (Utilities|FlowControl|Sequence
        (:then_0
          (Rendering|Material|SetScalarParameterValue _output_get "Cubemap Angle" (/ (+ (.yaw (Transformation|GetActorRotation)) (Variables|Lighting|GetSkybox%20Offset)) 3.6e+02) :!class /Script/Engine.MaterialInstanceDynamic))
        (:then_1
          (Rendering|Material|SetTextureParameterValue _output_get "Cubemap" _cubemap)
          (Class|SkyLightComponent|SetCubemap (Variables|Default|GetSkyLight) _cubemap))
        (:then_2
          (Rendering|Material|SetVectorParameterValue _output_get "Tint" (Variables|Lighting|GetTint) :!class /Script/Engine.MaterialInstanceDynamic))))
    (:then_2
      (Components|Arrow|SetArrowColor(LinearColor) (Variables|Default|GetLightDirection) (Rendering|Components|Light|GetLightColor (Variables|Default|GetDirectionalLight))))
    (:then_3
      (Transformation|SetRelativeLocation _colourcalibrator (Math|Vector|MakeVector 0.0 0.0 (.z (.BoxExtent (Collision|GetComponentBounds _colourcalibrator)))) false false)
      (Transformation|SetWorldRotation (Variables|Default|GetColourCalibrator) (Math|Rotator|MakeRotator 0.0 0.0 (Variables|Lighting|GetColour%20Calibrator%20Rotation)) false false))))